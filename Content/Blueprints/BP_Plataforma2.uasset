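; BP_Plataforma2 is a moving platform whose path is shaped by a spline and driven by an InterpToMovement component.
; The construction script turns the local origin and the next two spline points into relative control points, so the path supports exactly three stops.
; It also applies the Duration variable to the movement and stores a dynamic material instance of the platform mesh.
; The event graph holds only disabled placeholder events.
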(fn `UserConstructionScript`
  (bind _interptomovement (`self.InterpToMovement`))
  (set `InterpToMovementComponent.ControlPoints` (`|MakeArray` (make `InterpControlPoint` (0.0 0.0 0.0)) (make `InterpControlPoint` (`SplineComponent.GetLocationAtSplinePoint` (`self.Spline`) 1 "Local")) (make `InterpControlPoint` (`SplineComponent.GetLocationAtSplinePoint` (`self.Spline`) 2 "Local"))) _interptomovement)
  (set `InterpToMovementComponent.Duration` (`self.Duration`) _interptomovement)
  (bind _returnvalue (`PrimitiveComponent.CreateDynamicMaterialInstance` (`self.Plataforma`) 0 null "None"))
  (set `self.MaterialPlataforma` _returnvalue))