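; Elevator platform actor that moves when the third-person player character enters its Box trigger.
; The overlap activates InterpToMovement, stores the current location and restarts the Elevador timeline, whose output offsets the actor from that location without sweep.
; Each new overlap re-bases the motion on the current position.
; Spline-based control points, duration and dynamic material setup sit in unconnected construction script nodes that never run.
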(event `self.Box.OnComponentBeginOverlap`
  (params (OverlappedComponent :type "PrimitiveComponent Object Reference") (OtherActor :type "Actor Object Reference") (OtherComp :type "PrimitiveComponent Object Reference") (OtherBodyIndex :type Integer) (bFromSweep :type Boolean) (SweepResult :type "HitResult Structure (by ref)"))
  (cast `/Game/ThirdPerson/Blueprints/BP_ThirdPersonCharacter` OtherActor)
  (`ActorComponent.Activate` (`self.InterpToMovement`) false)
  (set `self.Posicion elevador` (`self.K2_GetActorLocation`))
  (bind (_direction _elevator) (`Timeline|Elevador` :!via `PlayFromStart`)
    (:`Update`
      (`self.K2_SetActorLocation` (+ _elevator (`self.Posicion elevador`))))))

(fn `UserConstructionScript`)