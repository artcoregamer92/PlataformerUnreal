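; A moving platform that starts travelling when the third-person character enters its trigger box, then gives way and falls.
; The construction script builds InterpToMovement control points from the spline's points, applies the Duration variable and creates a dynamic material for the mesh.
; On overlap it activates the movement, then after timed delays blackens a material parameter, plays a camera shake at the player, and finally enables physics on the platform.
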(event `self.Box.OnComponentBeginOverlap`
  (params (OverlappedComponent :type "PrimitiveComponent Object Reference") (OtherActor :type "Actor Object Reference") (OtherComp :type "PrimitiveComponent Object Reference") (OtherBodyIndex :type Integer) (bFromSweep :type Boolean) (SweepResult :type "HitResult Structure (by ref)"))
  (cast `/Game/ThirdPerson/Blueprints/BP_ThirdPersonCharacter` OtherActor)
  (`ActorComponent.Activate` (`self.InterpToMovement`) false)
  (`KismetSystemLibrary.Delay` 2.0)
  (`MaterialInstanceDynamic.SetVectorParameterValue` (`self.MaterialPlataform`) "Sample Texture" (struct :`A` 1.0))
  (`GameplayStatics.PlayWorldCameraShake` "/Game/Blueprints/BP_Shake.BP_Shake_C" (`self.K2_GetActorLocation` (`GameplayStatics.GetPlayerPawn` 0)) 500.0)
  (`KismetSystemLibrary.Delay` 1.0)
  (`PrimitiveComponent.SetSimulatePhysics` (`self.Plataforma`) true))

(fn `UserConstructionScript`
  (bind _interptomovement (`self.InterpToMovement`))
  (set `InterpToMovementComponent.ControlPoints` (`|MakeArray` (make `InterpControlPoint` (0.0 0.0 0.0)) (make `InterpControlPoint` (`SplineComponent.GetLocationAtSplinePoint` (`self.Spline`) 1 "Local")) (make `InterpControlPoint` (`SplineComponent.GetLocationAtSplinePoint` (`self.Spline`) 2 "Local")) (make `InterpControlPoint` (`SplineComponent.GetLocationAtSplinePoint` (`self.Spline`) 3 "Local")) (make `InterpControlPoint` (`SplineComponent.GetLocationAtSplinePoint` (`self.Spline`) 4 "Local"))) _interptomovement)
  (set `InterpToMovementComponent.Duration` (`self.Duration`) _interptomovement)
  (bind _returnvalue (`PrimitiveComponent.CreateDynamicMaterialInstance` (`self.Plataforma`) 0 "/Game/PolygonStarter/Materials/M_Polygon_Plane_02.M_Polygon_Plane_02" "None"))
  (set `self.MaterialPlataform` _returnvalue))