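; BP_Health is a trigger zone meant to restore the third-person character's health (VidaActual) while they stand inside its Box.
; Begin overlap caches the character and sets Detectado, which end overlap clears to stop healing.
; A short Delay loop adds a fixed amount to VidaActual only while it is below zero.
; The character's maximum health, VidaTotal, is fetched but unused, so it does not limit the loop.
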(event `self.Box.OnComponentBeginOverlap`
  (params (OverlappedComponent :type "PrimitiveComponent Object Reference") (OtherActor :type "Actor Object Reference") (OtherComp :type "PrimitiveComponent Object Reference") (OtherBodyIndex :type Integer) (bFromSweep :type Boolean) (SweepResult :type "HitResult Structure (by ref)"))
  (bind _as_bp_third_person_character (`self.As BP Third Person Character`))
  (bind _asbp_third_person_character (cast `/Game/ThirdPerson/Blueprints/BP_ThirdPersonCharacter` OtherActor))
  (set `self.As BP Third Person Character` _asbp_third_person_character)
  (set `self.Detectado` true)
  (if (and (< (`/Game/ThirdPerson/Blueprints/BP_ThirdPersonCharacter.VidaActual` (`self.As BP Third Person Character`)) 0.0) (`self.Detectado`)) :!label _label
    (set `/Game/ThirdPerson/Blueprints/BP_ThirdPersonCharacter.VidaActual` (+ (`/Game/ThirdPerson/Blueprints/BP_ThirdPersonCharacter.VidaActual` _as_bp_third_person_character) 2.0) _as_bp_third_person_character)
    (`KismetSystemLibrary.Delay` 0.01)
    (goto _label)))

(event `self.Box.OnComponentEndOverlap`
  (params (OverlappedComponent :type "PrimitiveComponent Object Reference") (OtherActor :type "Actor Object Reference") (OtherComp :type "PrimitiveComponent Object Reference") (OtherBodyIndex :type Integer))
  (cast `/Game/ThirdPerson/Blueprints/BP_ThirdPersonCharacter` OtherActor)
  (set `self.Detectado` false))

(fn `UserConstructionScript`)